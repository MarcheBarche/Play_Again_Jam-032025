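; BP_Player is the player-controlled actor, with first-person-style movement, camera look and projectile shooting driven by Enhanced Input.
; On BeginPlay it adds the IMC_Player mapping context and creates a HUD widget filled once with name, Life and Rage.
; Move input follows the actor's axes, look input drives control rotation copied to the camera, and shooting spawns BP_Projectile at ShootingPoint along that rotation.
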(event Input|EnhancedActionEvents|EnhancedInputActionIA_PlayerMovement
  (params (ActionValue :type Vector%202D%20Structure) (ElapsedSeconds :type Float%20%28double-precision%29) (TriggeredSeconds :type Float%20%28double-precision%29) (InputAction :type Input%20Action%20Object%20Reference :default "/Game/Input/IA_PlayerMovement.IA_PlayerMovement"))
  (Pawn|Input|AddMovementInput (* (Transformation|GetActorRightVector) (Variables|Default|Getspeed)) (.x ActionValue) false)
  (Pawn|Input|AddMovementInput (* (Transformation|GetActorForwardVector) (Variables|Default|Getspeed)) (.y ActionValue) false))

(event Input|EnhancedActionEvents|EnhancedInputActionIA_CameraRotation
  (params (ActionValue :type Vector%202D%20Structure) (ElapsedSeconds :type Float%20%28double-precision%29) (TriggeredSeconds :type Float%20%28double-precision%29) (InputAction :type Input%20Action%20Object%20Reference :default "/Game/Input/IA_CameraRotation.IA_CameraRotation"))
  (Pawn|Input|AddControllerYawInput (.x ActionValue))
  (Pawn|Input|AddControllerPitchInput (.y ActionValue))
  (Transformation|SetWorldRotation (Variables|Default|GetCamera) (Pawn|GetControlRotation :!class /Script/Engine.Pawn) false false))

(event Input|EnhancedActionEvents|EnhancedInputActionIA_PlayerShoot
  (params (ActionValue :type Boolean) (ElapsedSeconds :type Float%20%28double-precision%29) (TriggeredSeconds :type Float%20%28double-precision%29) (InputAction :type Input%20Action%20Object%20Reference :default "/Game/Input/IA_PlayerShoot.IA_PlayerShoot"))
  (Development|PrintText "Shoot")
  (Game|SpawnActorfromClass "/Game/BP/BP_Projectile.BP_Projectile_C" (Math|Transform|MakeTransform (.location (Transformation|GetWorldTransform (Variables|Default|GetShootingPoint))) (Pawn|GetControlRotation :!class /Script/Engine.Pawn) "1.000000,1.000000,1.000000") "Undefined" "OverrideRootScale" 0 0))

(event EventBeginPlay
  (Input|AddMappingContext (PlayerController|LocalPlayerSubsystems|GetEnhancedInputLocalPlayerSubsystem (Game|GetPlayerController 0)) "/Game/Input/IMC_Player.IMC_Player" 0 "(bIgnoreAllPressedKeysUntilRelease=True,bForceImmediately=False,bNotifyUserSettings=False)")
  (CallFunction|InitUI))

(fn ConstructionScript)

(fn InitUI
  (bind _returnvalue (Game|GetPlayerController 0))
  (bind _returnvalue_2 (UserInterface|CreateWidget "/Game/UI/WB_Player.WB_Player_C" _returnvalue))
  (Utilities|FlowControl|Sequence
    (:then_0
      (Variables|/Script/UMG.TextBlock|SetText (Variables|/Game/UI/WB_Player.WB_Player_C|GetTextName _returnvalue_2) (Utilities|Text|FormatText "Name: {a}" (Utilities|GetDisplayName _returnvalue))))
    (:then_1
      (Variables|/Script/UMG.TextBlock|SetText (Variables|/Game/UI/WB_Player.WB_Player_C|GetTextLife _returnvalue_2) (Utilities|Text|FormatText "Life: {a}" (Variables|Default|GetLife))))
    (:then_2
      (Variables|/Script/UMG.TextBlock|SetText (Variables|/Game/UI/WB_Player.WB_Player_C|GetTextRage _returnvalue_2) (Utilities|Text|FormatText "Rage: {a}" (Variables|Default|GetRage))))
    (:then_3
      (UserInterface|Viewport|AddtoViewport _returnvalue_2 0))))